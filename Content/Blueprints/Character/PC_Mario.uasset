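; Player controller for Mario that routes player input to the Mario character.
; On BeginPlay it casts player character 0 to C_Mario and caches the reference.
; Movement and look axes and jump press and release are forwarded to matching functions on that character, which owns the actual behaviour.
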(event EventBeginPlay
  (bind _asc_mario (Utilities|Casting|CastToC_Mario (Game|GetPlayerCharacter 0)))
  (Variables|Default|SetMarioRef _asc_mario))

(event Input|ActionEvents|InputActionJump
  (params (Key :type Key%20Structure :default "None"))
  (bind _marioref (Variables|Default|GetMarioRef))
  (:Pressed
    (Default|DoJump _marioref true))
  (:Released
    (Default|DoJump _marioref false)))

(event Input|AxisEvents|InputAxisMoveForwardBackward
  (params (AxisValue :type Float%20%28single-precision%29))
  ;[1 1 1] Move
  (Default|MoveForwardBackward (Variables|Default|GetMarioRef) AxisValue))

(event Input|AxisEvents|InputAxisMoveRightLeft
  (params (AxisValue :type Float%20%28single-precision%29))
  ;[1 1 1] Move
  (Default|MoveRightLeft (Variables|Default|GetMarioRef) AxisValue))

(event Input|AxisEvents|InputAxisLookUpDown
  (params (AxisValue :type Float%20%28single-precision%29))
  ;[1 1 1] Look
  (Default|LookUpDown (Variables|Default|GetMarioRef) AxisValue))

(event Input|AxisEvents|InputAxisLookRightLeft
  (params (AxisValue :type Float%20%28single-precision%29))
  ;[1 1 1] Look
  (Default|LookRightLeft (Variables|Default|GetMarioRef) AxisValue))

(fn ConstructionScript)